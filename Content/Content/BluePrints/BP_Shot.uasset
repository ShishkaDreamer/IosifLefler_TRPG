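; BP_Shot is a short-lived shot actor that deals magic damage to whatever overlaps its Sphere.
; FvInit stores the damage and shrinks the mesh.
; On BeginPlay it keeps Sphere collision off briefly before enabling it, while a parallel timer destroys the actor after a few seconds.
; An overlap sends the damage to the other actor via the MakeMagicDMG message, then destroys the shot.
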(event `self.ReceiveBeginPlay`
  (bind _sphere (`self.Sphere`))
  (`|ExecutionSequence`
    (:`then_0`
      (`KismetSystemLibrary.Delay` 4.0)
      (`self.K2_DestroyActor`))
    (:`then_1`
      (`PrimitiveComponent.SetCollisionEnabled` _sphere "NoCollision")
      (`KismetSystemLibrary.Delay` 0.3)
      (`PrimitiveComponent.SetCollisionEnabled` _sphere "QueryAndPhysics"))))

(event `self.Sphere.OnComponentBeginOverlap`
  (params (OverlappedComponent :type "PrimitiveComponent Object Reference") (OtherActor :type "Actor Object Reference") (OtherComp :type "PrimitiveComponent Object Reference") (OtherBodyIndex :type Integer) (bFromSweep :type Boolean) (SweepResult :type "HitResult Structure (by ref)"))
  (message `/Game/Content/BluePrints/Main/BP_Iterface.MakeMagicDMG` OtherActor (`self.Dmg`))
  (`self.K2_DestroyActor`))

(fn `fv Init`
  (params (DMG :type "Float (double-precision)"))
  (set `self.Dmg` DMG)
  (`SceneComponent.SetWorldScale3D` (`self.StaticMesh`) (0.3 0.3 0.3)))

(fn `UserConstructionScript`)