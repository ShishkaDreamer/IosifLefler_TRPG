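; BP_Parameters holds health state and provides functions to apply damage and healing.
; FvGetDmg subtracts positive damage and prints a debug message, while FvGetHeal adds healing without checking its sign.
; Both route the result through FvSetHealth, which clamps CurrentHealth between zero and MaxHealth.
; The event graph has no active logic, and nothing here handles death at zero health.
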(fn `fv GetDmg`
  (params (DMG :type "Float (double-precision)"))
  (if (> DMG 0.0)
    (`self.fv SetHealth` (`KismetMathLibrary.FMax` (- (`self.CurrentHealth`) DMG)))
    (`KismetSystemLibrary.PrintString` "DMG got")))

(fn `fv GetHeal`
  (params (Heal :type "Float (double-precision)"))
  (`self.fv SetHealth` (`KismetMathLibrary.FMin` (+ Heal (`self.CurrentHealth`)) (`self.MaxHealth`))))

(fn `fv SetHealth`
  (params (Health :type "Float (double-precision)"))
  (set `self.CurrentHealth` (`KismetMathLibrary.FClamp` Health 0.0 (`self.MaxHealth`))))