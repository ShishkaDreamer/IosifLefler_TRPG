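; BP_Character is a character Blueprint that exposes simple move and jump functions and sets up health when play begins.
; On BeginPlay, FvInit passes MaxHealth from BPParameters into its FvSetHealth function.
; FvMove stores the given vector and feeds it to CharacterMovement as input.
; FvJump applies a large upward force through CharacterMovement instead of calling the built-in Jump.
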(event `self.ReceiveBeginPlay`
  (`self.fv Init`))

(fn `fv Init`
  (bind _bp_parameters (`self.BP_Parameters`))
  (`/Game/Content/BluePrints/Main/BP_Parameters.fv SetHealth` _bp_parameters (`/Game/Content/BluePrints/Main/BP_Parameters.MaxHealth` _bp_parameters)))

(fn `fv Jump`
  (`CharacterMovementComponent.AddForce` (`self.CharacterMovement`) (0.0 0.0 3000000.0)))

(fn `fv Move`
  (params (`@MoveVector1` :type "Vector Structure"))
  (locals (`@MoveVector` :type "Vector Structure" :default (0.0 0.0 0.0)))
  (bind _output_get (set `local.@MoveVector` `@MoveVector1`))
  (`PawnMovementComponent.AddInputVector` (`self.CharacterMovement`) _output_get false))

(fn `UserConstructionScript`)